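; BP_Enemy is an enemy actor that turns toward the player and fires a single bullet when play begins.
; On BeginPlay it casts player character 0 to Ue4ASP_Character and sets its rotation once to look at that character.
; After a short delay it spawns a BP_Bullet at the BulletSpawn component's world transform, with no repeated tracking or firing.
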(event EventBeginPlay
  (bind _asue_4asp_character (Utilities|Casting|CastToUe4ASP_Character (Game|GetPlayerCharacter 0)))
  (Utilities|FlowControl|Sequence
    (:then_0
      (Transformation|SetActorRotation (Math|Rotator|FindLookatRotation (Transformation|GetActorLocation) (Transformation|GetActorLocation _asue_4asp_character))))
    (:then_1
      (Utilities|FlowControl|Delay 0.5)
      (Game|SpawnActorfromClass "/Game/Items/Weapons/BP_Bullet.BP_Bullet_C" (Transformation|GetWorldTransform (Variables|Default|GetBulletSpawn)) "Undefined" 0 "0.000000,0.000000,0.000000" 0))))

(event Collision|EventActorBeginOverlap
  (params (OtherActor :type Actor%20Object%20Reference)))

(event EventTick
  (params (DeltaSeconds :type Float%20%28single-precision%29)))

(fn ConstructionScript)