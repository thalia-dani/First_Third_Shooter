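; BP_Item is an item actor that shows an on-screen interaction prompt while a player is in interaction range.
; The range-enter event creates an Interaction_Widget in a screen-space widget component, if none exists, and the range-exit event destroys that component.
; GetInteractionText and InteractionTextAttach supply the prompt's text and attach point, defaulting to a generic label and the root component.
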(event EventBeginPlay)

(event Collision|EventActorBeginOverlap
  (params (OtherActor :type Actor%20Object%20Reference)))

(event EventTick
  (params (DeltaSeconds :type Float%20%28single-precision%29)))

(event EventOnInteractionRangeEnter
  (params (Player :type Ue%204ASP%20Character%20Object%20Reference))
  (Variables|Default|GetInteractionWidgetComponent
    (:then)
    (:else
      (bind _returnvalue (Game|ConstructObjectfromClass "/Game/InteractInterface/Interaction_Widget.Interaction_Widget_C" (.AsPlayer%20Controller (Utilities|Casting|CastToPlayerController (Pawn|GetController Player))) (CallFunction|GetInteractionText)))
      (bind _returnvalue_2 (AddComponent|AddWidgetComponent false))
      (bind _output_get (Variables|Default|SetInteractionWidgetComponent _returnvalue_2))
      (UserInterface|SetWidget _output_get _returnvalue)
      (Class|WidgetComponent|SetWidgetSpace _output_get "Screen")
      (Class|WidgetComponent|SetDrawatDesiredSize _output_get true)
      (Collision|SetCollisionEnabled _output_get "NoCollision")
      (Transformation|AttachComponentToComponent _output_get (Private|InteractionTextAttach) "None" "SnapToTarget" "SnapToTarget" "SnapToTarget" true))))

(event EventOnInteractionRangeExit
  (bind _interactionwidgetcomponent (Variables|Default|GetInteractionWidgetComponent)
    (:then
      (Components|DestroyComponent _interactionwidgetcomponent))
    (:else)))

(fn ConstructionScript)

(fn GetInteractionText
  (return "Interact"))

(fn InteractionTextAttach
  (return (Variables|Default|GetDefaultSceneRoot)))