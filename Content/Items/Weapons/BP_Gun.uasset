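; BP_Gun is an interactable weapon that the player can pick up, fire, reload and drop.
; A Dropped/Equipped state switches mesh physics and collision, starting Dropped and becoming Equipped when interaction passes it to the player.
; Fire spawns a bullet and muzzle effect at the muzzle socket, aiming toward a distant point along the camera's forward vector.
; Reload refills from reserve ammo, discarding any rounds left in the clip.
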(event Collision|EventActorBeginOverlap
  (params (OtherActor :type Actor%20Object%20Reference))
  (|CallParentFunction OtherActor) ; This node is disabled and will not be called.\nDrag off pins to build functionality.
)

(event EventTick
  (params (DeltaSeconds :type Float%20%28single-precision%29))
  (|CallParentFunction DeltaSeconds) ; This node is disabled and will not be called.\nDrag off pins to build functionality.
)

(event EventOnInteractedPlayer
  (params (Player :type Ue%204ASP%20Character%20Object%20Reference))
  (Default|PickUpWeapon Player self)
  (Private|SetGunState "NewEnumerator1"))

(event EventBeginPlay
  (Private|SetGunState "NewEnumerator0"))

(fn ConstructionScript
  (|CallParentFunction))

(fn GetInteractionText
  (return "Pick Up"))

(fn InteractionTextAttach
  (return (Variables|Default|GetSkeletalMesh)))

(fn SetGunState
  (params (New%20Gun%20State :type EnumGunState%20Enum :default "NewEnumerator0"))
  (bind _skeletalmesh (Variables|Default|GetSkeletalMesh))
  (bind _skeletalmesh_2 (Variables|Default|GetSkeletalMesh))
  (bind _output_get (Variables|Private|SetGun%20State New%20Gun%20State))
  (switch Utilities|FlowControl|Switch|SwitchonEnumGunState _output_get
    (:NewEnumerator0
      (Collision|SetCollisionProfileName (Variables|Default|GetSphere) "OverlapAllDynamic" true :!class /Script/Engine.PrimitiveComponent)
      (Physics|SetSimulatePhysics _skeletalmesh_2 true)
      (Collision|SetCollisionProfileName _skeletalmesh_2 "DropWeapon" true :!class /Script/Engine.PrimitiveComponent))
    (:NewEnumerator1
      (Collision|SetCollisionProfileName (Variables|Default|GetSphere) "NoCollision" true :!class /Script/Engine.PrimitiveComponent)
      (Physics|SetSimulatePhysics _skeletalmesh false)
      (Collision|SetCollisionProfileName _skeletalmesh "NoCollision" true :!class /Script/Engine.PrimitiveComponent)
      (Transformation|ResetRelativeTransform _skeletalmesh))))

(fn Drop
  (Private|SetGunState "NewEnumerator0"))

(fn Fire
  (params (PlayerCamera :type Camera%20Component%20Object%20Reference))
  (bind _skeletalmesh (Variables|Default|GetSkeletalMesh))
  (bind _returnvalue (Transformation|GetSocketLocation _skeletalmesh "b_gun_muzzleflash"))
  (Game|SpawnActorfromClass "/Game/Items/Weapons/BP_Bullet.BP_Bullet_C" (Math|Transform|MakeTransform _returnvalue "0, 0, 0" "1,1,1") "Undefined" 0 (* (Math|Vector|Normalize (- (+ (Transformation|GetWorldLocation PlayerCamera) (* (Math|Vector|GetForwardVector PlayerCamera) 1e+04)) _returnvalue)) 1e+04) 0)
  (Game|SpawnActorfromClass "/Game/Items/Weapons/BP_Muzzle.BP_Muzzle_C" (Math|Transform|MakeTransform _returnvalue "0, 0, 0" "1,1,1") "Undefined" 0 0)
  (Variables|Default|SetAmmo (- (Variables|Default|GetAmmo) 1)))

(fn Reload
  (if (not (== (Variables|Default|GetAmmo) (Variables|Default|GetClipSize)))
    (if (> (Variables|Default|GetMaxAmmo) (Variables|Default|GetClipSize))
      (Variables|Default|SetAmmo (Variables|Default|GetClipSize))
      (Variables|Default|SetMaxAmmo (- (Variables|Default|GetMaxAmmo) (Variables|Default|GetClipSize)))
      (else
        (Variables|Default|SetAmmo (Variables|Default|GetMaxAmmo))
        (Variables|Default|SetMaxAmmo 0)))))